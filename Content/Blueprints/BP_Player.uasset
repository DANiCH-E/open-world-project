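; Third-person player character with Enhanced Input movement and look, a toggleable rifle and aiming.
; Aiming switches to controller-facing strafe movement, while a timeline pulls the spring arm in and raises it.
; With the rifle equipped, holding fire loops a timer that plays the fire montage.
; Montage notifies trigger a muzzle line trace with impact particles, plus muzzle flash, camera shake and sound; no damage is applied.
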(event `self.ReceiveBeginPlay`
  (`EnhancedInputSubsystemInterface.AddMappingContext` (pcsubsystem `EnhancedInputLocalPlayerSubsystem` (`GameplayStatics.GetPlayerController` 0)) "/Game/Input/IMC_PlayerInput.IMC_PlayerInput" 0 (struct)))

(event `EnhancedInput|/Game/Input/IA_Move`
  (params (ActionValue :type "Vector2D Structure") (ElapsedSeconds :type "Float (double-precision)") (TriggeredSeconds :type "Float (double-precision)") (InputAction :type "InputAction Object Reference" :default "/Game/Input/IA_Move.IA_Move"))
  (bind (_returnvalue_roll _returnvalue_pitch _returnvalue_yaw) (`KismetMathLibrary.BreakRotator` (`self.GetControlRotation`)))
  (bind (_returnvalue_roll_2 _returnvalue_pitch_2 _returnvalue_yaw_2) (`KismetMathLibrary.BreakRotator` (`self.GetControlRotation`)))
  ;[1 1 1] Movement
  (:`Triggered`
    (`self.AddMovementInput` (`KismetMathLibrary.GetRightVector` (`KismetMathLibrary.MakeRotator` _returnvalue_roll 0.0 _returnvalue_yaw)) ActionValue_X)
    (`self.AddMovementInput` (`KismetMathLibrary.GetForwardVector` (`KismetMathLibrary.MakeRotator` _returnvalue_roll_2 0.0 _returnvalue_yaw_2)) ActionValue_Y)))

(event `EnhancedInput|/Game/Input/IA_Look`
  (params (ActionValue :type "Vector2D Structure") (ElapsedSeconds :type "Float (double-precision)") (TriggeredSeconds :type "Float (double-precision)") (InputAction :type "InputAction Object Reference" :default "/Game/Input/IA_Look.IA_Look"))
  ;[1 1 1] Looking
  (:`Triggered`
    (`self.AddControllerYawInput` ActionValue_X)
    (`self.AddControllerPitchInput` (* ActionValue_Y -1.0))))

(event `EnhancedInput|/Game/Input/IA_Equip_Rifle`
  (params (ActionValue :type Boolean) (ElapsedSeconds :type "Float (double-precision)") (TriggeredSeconds :type "Float (double-precision)") (InputAction :type "InputAction Object Reference" :default "/Game/Input/IA_Equip_Rifle.IA_Equip_Rifle"))
  ;[1 1 1] Rifle Equipment
  (:`Started`
    (if (not (`self.RifleEquipped`))
      (set `self.RifleEquipped` true)
      (`KismetSystemLibrary.Delay` 0.5)
      (`SceneComponent.SetVisibility` (`self.Rifle`) true false)
      (else
        (set `self.RifleEquipped` false)
        (`KismetSystemLibrary.Delay` 0.5)
        (`SceneComponent.SetVisibility` (`self.Rifle`) false false)))))

(event `EnhancedInput|/Game/Input/IA_Aim`
  (params (ActionValue :type Boolean) (ElapsedSeconds :type "Float (double-precision)") (TriggeredSeconds :type "Float (double-precision)") (InputAction :type "InputAction Object Reference" :default "/Game/Input/IA_Aim.IA_Aim"))
  (bind _springarm (`self.SpringArm`))
  (bind (_socketoffset_x _socketoffset_y) (`KismetMathLibrary.BreakVector` (`SpringArmComponent.SocketOffset` _springarm)))
  ;[1 1 1] Aim
  (:`Started`
    (set `self.IsAiming` true)
    (`self.Set Strafe Movement`)
    (bind (_direction _aim_length) (`Timeline|Aim` :!label _label)
      (:`Update`
        (set `SpringArmComponent.TargetArmLength` (`KismetMathLibrary.Lerp` 300.0 150.0 _aim_length) (`self.SpringArm`))
        (set `SpringArmComponent.SocketOffset` (`KismetMathLibrary.MakeVector` _socketoffset_x _socketoffset_y (`KismetMathLibrary.Lerp` 0.0 25.0 _aim_length)) _springarm))))
  (:`Completed`
    (set `self.IsAiming` false)
    (`self.Set Free Movement`)
    (goto _label :!via `Reverse`)))

(event `Set Strafe Movement`
  (bind _charactermovement (`self.CharacterMovement`))
  ;[1 1 1] Aim
  (set `CharacterMovementComponent.bOrientRotationToMovement` false _charactermovement)
  (set `CharacterMovementComponent.bUseControllerDesiredRotation` true _charactermovement))

(event `Set Free Movement`
  (bind _charactermovement (`self.CharacterMovement`))
  ;[1 1 1] Aim
  (set `CharacterMovementComponent.bOrientRotationToMovement` true _charactermovement)
  (set `CharacterMovementComponent.bUseControllerDesiredRotation` false _charactermovement))

(event `EnhancedInput|/Game/Input/IA_Fire`
  (params (ActionValue :type Boolean) (ElapsedSeconds :type "Float (double-precision)") (TriggeredSeconds :type "Float (double-precision)") (InputAction :type "InputAction Object Reference" :default "/Game/Input/IA_Fire.IA_Fire"))
  ;[1 1 1] Firing
  (:`Started`
    (if (`self.RifleEquipped`)
      (bind _returnvalue (`KismetSystemLibrary.K2_SetTimerDelegate` (delegate `Fire Rifle`) 0.1 true))))
  (:`Completed`
    (`KismetSystemLibrary.K2_ClearAndInvalidateTimerHandle` _returnvalue)))

(event `Fire Rifle`
  (bind (_returnvalue_location _returnvalue_rotation) (`KismetMathLibrary.BreakTransform` (`SceneComponent.GetSocketTransform` (`self.Rifle`) "Muzzle" "RTS_World")))
  (bind (_returnvalue_location_2 _returnvalue_rotation_2) (`KismetMathLibrary.BreakTransform` (`SceneComponent.GetSocketTransform` (`self.Rifle`) "Muzzle" "RTS_World")))
  ;[1 1 1] Firing
  (`|PlayMontage` (`self.Mesh`) "/Game/Characters/Animations/Rifle/Fire_Rifle_Montage.Fire_Rifle_Montage"
    (:`OnNotifyBegin`
      (`|ExecutionSequence`
        (:`then_0`
          (bind (_outhit _returnvalue) (`KismetSystemLibrary.LineTraceSingle` _returnvalue_location_2 (+ _returnvalue_location_2 (* (`KismetMathLibrary.GetForwardVector` _returnvalue_rotation_2) 5000.0)) "TraceTypeQuery1"))
          (if _returnvalue
            (bind (_bblockinghit _binitialoverlap _time _distance _location _impactpoint _normal) (`GameplayStatics.BreakHitResult` _outhit))
            (`GameplayStatics.SpawnEmitterAtLocation` "/Game/InfinityBladeEffects/Effects/FX_Monsters/FX_Monster_Troll/death/P_TrollDeathImpact.P_TrollDeathImpact" _impactpoint (`KismetMathLibrary.MakeRotFromX` _normal) (0.3 0.3 0.3) true "AutoRelease")))
        (:`then_1`
          (`GameplayStatics.SpawnEmitterAttached` "/Game/InfinityBladeEffects/Effects/FX_Monsters/FX_Monster_Gruntling/Master/P_BackPack_MuzzleFlash.P_BackPack_MuzzleFlash" (`self.Rifle`) "Muzzle" _returnvalue_location _returnvalue_rotation (0.3 0.3 0.3) "KeepWorldPosition" true "AutoRelease")
          (`GameplayStatics.PlayWorldCameraShake` "/Game/Blueprints/BP_RifleFireCameraShake.BP_RifleFireCameraShake_C" (`self.K2_GetActorLocation`) 0.0 500.0)
          (`GameplayStatics.PlaySoundAtLocation` "/Game/Audio/MS_RifleFire.MS_RifleFire" (`self.K2_GetActorLocation`) (struct) 1.0 1.0 0.0 null null null null))))))

(fn `UserConstructionScript`)